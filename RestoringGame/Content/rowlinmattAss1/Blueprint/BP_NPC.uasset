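; BP_NPC is a Paper2D NPC that walks back and forth along world X between fixed bounds either side of the origin.
; Each tick it reverses direction past a bound, rotates the sprite to match and feeds movement input that way.
; Tick also picks the jump, run or stance flipbook from State and velocity, though nothing here sets State.
; BeginPlay enables replication on the sprite component.
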(event `self.ReceiveBeginPlay`
  (`ActorComponent.SetIsReplicated` (`self.Sprite`) true))

(event `UpdateAnimation`
  ;[1 1 1] Handle Animation
  (if (`|EnumEquality` (`self.State`) "NewEnumerator2")
    (`PaperFlipbookComponent.SetFlipbook` (`self.Sprite`) "/Game/rowlinmattAss1/Sprites/Character/A_Jump.A_Jump")
    (else
      (`PaperFlipbookComponent.SetFlipbook` (`self.Sprite`) (select `bool` (> (`KismetMathLibrary.VSize` (`self.GetVelocity`)) 0.0) :`false` "/Game/rowlinmattAss1/Sprites/Character/A_Stance.A_Stance" :`true` "/Game/rowlinmattAss1/Sprites/Character/A_Run.A_Run" :!type "PaperFlipbook Object Reference")))))

(event `self.ReceiveTick`
  (params (DeltaSeconds :type "Float (single-precision)"))
  (bind _bismovingright (`self.bisMovingRight`))
  (bind _x (.x (`SceneComponent.K2_GetComponentLocation` (`self.Sprite`))))
  ;[1 1 1] Tick - Updates animation
  (`self.UpdateAnimation`)
  (if (> _x 300.0)
    (set `self.bisMovingRight` false))
  (if (< _x -300.0)
    (set `self.bisMovingRight` true))
  (`SceneComponent.K2_SetRelativeRotation` (`self.Sprite`) (`KismetMathLibrary.SelectRotator` (struct) (struct :`Yaw` 180.0) _bismovingright) false false)
  (`self.AddMovementInput` (`KismetMathLibrary.SelectVector` (1.0 0.0 0.0) (-1.0 0.0 0.0) _bismovingright)))

(fn `UserConstructionScript`)